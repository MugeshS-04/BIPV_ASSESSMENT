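; Selection Blueprint that inspects Cesium-style feature metadata on whatever the camera faces and shows the mouse cursor on BeginPlay.
; Left click runs a Visibility line trace along the camera's forward vector, not through the cursor position, with debug drawing.
; The hit's property table values for feature ID set 0 print on screen as key:value strings.
; An unconnected StaticMeshActor location printout is leftover and never runs.
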(event EventBeginPlay
  (Variables|Default|SetbShowMouseCursor true))

(event EventTick
  (params (DeltaSeconds :type Float%20%28single-precision%29)))

(event Input|MouseEvents|LeftMouseButton
  (params (Key :type Key%20Structure))
  (bind _returnvalue (Game|GetPlayerCameraManager 0))
  (bind _returnvalue_2 (Camera|GetCameraLocation _returnvalue))
  (:Pressed
    (bind _outhit (Collision|LineTraceByChannel _returnvalue_2 (+ (* (Math|Vector|GetForwardVector (Camera|GetCameraRotation _returnvalue)) 1e+04) _returnvalue_2) "TraceTypeQuery1" false 0 "ForDuration"))
    (bind _keys (Utilities|Map|Keys (Class|CesiumMetadataValueBlueprintLibrary|GetValuesasStrings (Class|CesiumMetadataPickingBlueprintLibrary|GetPropertyTableValuesfromHit _outhit))))
    (for _array_element _keys
      (Development|PrintString (Utilities|String|Append _array_element ": " (.Value (Utilities|Map|Find (Class|CesiumMetadataValueBlueprintLibrary|GetValuesasStrings (Class|CesiumMetadataPickingBlueprintLibrary|GetPropertyTableValuesfromHit _outhit)) _array_element)))))))

(fn ConstructionScript)