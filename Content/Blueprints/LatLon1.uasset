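; Click-to-geolocate Blueprint that picks a world point on a Cesium globe and can query Solcast solar radiation for it.
; Left click traces along the camera's forward vector, not the cursor, and converts the hit through the default georeference, storing longitude (X) in LatClick and latitude (Y) in LonClick.
; HTTP2 sends those values to Solcast and prints the JSON response; nothing here calls it.
; Feature-metadata readout is disconnected and GetGhi is empty.
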(event Custom|HTTP2
  (bind _lat_click (Variables|Default|GetLat_Click))
  (bind _lon_click (Variables|Default|GetLon_Click))
  (bind _result (Utilities|Text|FormatText "https://api.solcast.com.au/world_radiation/estimated_actuals?latitude={0}&longitude={1}&output_parameters=ghi,dni,dhi&hours=24&format=json&api_key=1poKEkVfa7q3DJPl-qxUAQoqh90Ddqnw" _lat_click _lon_click))
  (bind _returnvalue (Utilities|String|ToString(Text) _result))
  (Variables|Default|Seturl _returnvalue)
  (bind _result_body (|HttpRequest _returnvalue "Get" (|MakeRequestHeader "Json"))
    (:On%20Success
      (Development|PrintString _result_body))))

(event EventBeginPlay
  (Variables|Default|SetbShowMouseCursor true))

(event EventTick
  (params (DeltaSeconds :type Float%20%28single-precision%29)))

(event Input|MouseEvents|LeftMouseButton
  (params (Key :type Key%20Structure :default "None"))
  (bind _returnvalue (Game|GetPlayerCameraManager 0))
  (bind _returnvalue_2 (Camera|GetCameraLocation _returnvalue))
  (:Pressed
    (bind _outhit (Collision|LineTraceByChannel _returnvalue_2 (+ (* (Math|Vector|GetForwardVector (Camera|GetCameraRotation _returnvalue)) 1e+04) _returnvalue_2) "TraceTypeQuery1" false 0 "ForDuration"))
    (bind _returnvalue_3 (Class|CesiumGeoreference|GetDefaultGeoreference))
    (Variables|Default|SetLat_Click (.X (Class|KismetMathLibrary|BreakVector3f (Class|CesiumGeoreference|TransformUnrealPositiontoLongitudeLatitudeHeight _returnvalue_3 (.ImpactPoint (Collision|BreakHitResult _outhit))))))
    (Development|PrintString (Utilities|String|ToString(Float) (.X (Class|KismetMathLibrary|BreakVector3f (Class|CesiumGeoreference|TransformUnrealPositiontoLongitudeLatitudeHeight _returnvalue_3 (.ImpactPoint (Collision|BreakHitResult _outhit)))))))
    (Variables|Default|SetLon_Click (.Y (Class|KismetMathLibrary|BreakVector3f (Class|CesiumGeoreference|TransformUnrealPositiontoLongitudeLatitudeHeight _returnvalue_3 (.ImpactPoint (Collision|BreakHitResult _outhit))))))
    (Development|PrintString (Utilities|String|ToString(Float) (.Y (Class|KismetMathLibrary|BreakVector3f (Class|CesiumGeoreference|TransformUnrealPositiontoLongitudeLatitudeHeight _returnvalue_3 (.ImpactPoint (Collision|BreakHitResult _outhit)))))))))

(fn ConstructionScript)

(fn GetGhi)