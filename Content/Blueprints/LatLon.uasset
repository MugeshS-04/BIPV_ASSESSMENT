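; LatLon picks geographic coordinates from Cesium feature metadata and can query Solcast for solar radiation estimates there.
; Left click traces along camera forward, not the cursor, then stores and prints the hit's Height, Longitude and Latitude properties.
; LatClick receives Longitude and LonClick Latitude, so the query coordinates are swapped.
; HTTP_Request, not called here, prints the JSON GHI/DNI/DHI response using a hardcoded API key; GetGhi is empty.
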(event Custom|HTTP_Request
  (bind _lat_click (Variables|Default|GetLat_Click))
  (bind _lon_click (Variables|Default|GetLon_Click))
  (bind _result (Utilities|Text|FormatText "https://api.solcast.com.au/world_radiation/estimated_actuals?latitude={0}&longitude={1}&output_parameters=ghi,dni,dhi&hours=24&format=json&api_key=DqLqypnKD5rCC_LBZYbGaUkcQiQqKT6f" _lat_click _lon_click))
  (bind _returnvalue (Utilities|String|ToString(Text) _result))
  (Variables|Default|Seturl _returnvalue)
  (bind _result_body (|HttpRequest _returnvalue "Get" (|MakeRequestHeader "Json"))
    (:On%20Success
      (Development|PrintString _result_body))))

(event EventBeginPlay
  (Variables|Default|SetbShowMouseCursor true))

(event EventTick
  (params (DeltaSeconds :type Float%20%28single-precision%29)))

(event Input|MouseEvents|LeftMouseButton
  (params (Key :type Key%20Structure :default "None"))
  (bind _returnvalue (Game|GetPlayerCameraManager 0))
  (bind _returnvalue_2 (Camera|GetCameraLocation _returnvalue))
  (:Pressed
    (bind _outhit (Collision|LineTraceByChannel _returnvalue_2 (+ (* (Math|Vector|GetForwardVector (Camera|GetCameraRotation _returnvalue)) 1e+04) _returnvalue_2) "TraceTypeQuery1" false 0 "ForDuration"))
    (bind _returnvalue_3 (Class|CesiumGeoreference|GetDefaultGeoreference))
    (Variables|Default|SetHeight_Click (Math|Conversions|ToFloat(Integer) (.Value (Utilities|Map|Find (Class|CesiumMetadataValueBlueprintLibrary|GetValuesasStrings (Class|CesiumMetadataPickingBlueprintLibrary|GetPropertyTableValuesfromHit _outhit)) (Variables|Default|GetHeight)))))
    (Development|PrintString "Height:")
    (Development|PrintString (.Value (Utilities|Map|Find (Class|CesiumMetadataValueBlueprintLibrary|GetValuesasStrings (Class|CesiumMetadataPickingBlueprintLibrary|GetPropertyTableValuesfromHit _outhit)) (Variables|Default|GetHeight))))
    (Variables|Default|SetLat_Click (Math|Conversions|ToFloat(Integer) (.Value (Utilities|Map|Find (Class|CesiumMetadataValueBlueprintLibrary|GetValuesasStrings (Class|CesiumMetadataPickingBlueprintLibrary|GetPropertyTableValuesfromHit _outhit)) (Variables|Default|GetLongitude)))))
    (Development|PrintString "Longitude:")
    (Development|PrintString (.Value (Utilities|Map|Find (Class|CesiumMetadataValueBlueprintLibrary|GetValuesasStrings (Class|CesiumMetadataPickingBlueprintLibrary|GetPropertyTableValuesfromHit _outhit)) (Variables|Default|GetLongitude))))
    (Variables|Default|SetLon_Click (Math|Conversions|ToFloat(Integer) (.Value (Utilities|Map|Find (Class|CesiumMetadataValueBlueprintLibrary|GetValuesasStrings (Class|CesiumMetadataPickingBlueprintLibrary|GetPropertyTableValuesfromHit _outhit)) (Variables|Default|GetLatitude)))))
    (Development|PrintString "Latitude:")
    (Development|PrintString (.Value (Utilities|Map|Find (Class|CesiumMetadataValueBlueprintLibrary|GetValuesasStrings (Class|CesiumMetadataPickingBlueprintLibrary|GetPropertyTableValuesfromHit _outhit)) (Variables|Default|GetLatitude))))))

(fn ConstructionScript)

(fn GetGhi)